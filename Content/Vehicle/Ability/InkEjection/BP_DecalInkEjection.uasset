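; BP_DecalInkEjection is the ink decal actor for the vehicle ink ejection ability, colored to match its instigator.
; The construction script reads the owned gameplay tags from the instigator's Ability System Component and switches on the Color tag to set the matching decal material instance.
; All logic runs at construction, with no active BeginPlay or Tick.
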(event EventBeginPlay)

(event EventTick
  (params (DeltaSeconds :type Float%20%28single-precision%29)))

(fn ConstructionScript
  (bind _decal (Variables|Decal|GetDecal))
  (|SwitchGameplayTagContainer (GameplayTags|GetOwnedGameplayTags (Ability|GetAbilitySystemComponent (Variables|Actor|GetInstigator)) :!class /Script/GameplayTags.BlueprintGameplayTagLibrary)
    (:%28GameplayTags=%28%28TagName="Color.Blue"%29%29%29
      (Rendering|Components|Decal|SetDecalMaterial _decal "/Game/Vehicle/Ability/InkEjection/M/MI_Decal_Blue.MI_Decal_Blue"))
    (:%28GameplayTags=%28%28TagName="Color.Cyan"%29%29%29
      (Rendering|Components|Decal|SetDecalMaterial _decal "/Game/Vehicle/Ability/InkEjection/M/MI_Decal_cyan.MI_Decal_cyan"))
    (:%28GameplayTags=%28%28TagName="Color.Green"%29%29%29
      (Rendering|Components|Decal|SetDecalMaterial _decal "/Game/Vehicle/Ability/InkEjection/M/MI_Decal_Green.MI_Decal_Green"))
    (:%28GameplayTags=%28%28TagName="Color.Orange"%29%29%29
      (Rendering|Components|Decal|SetDecalMaterial (Variables|Decal|GetDecal) "/Game/Vehicle/Ability/InkEjection/M/MI_Decal_Orange.MI_Decal_Orange"))
    (:%28GameplayTags=%28%28TagName="Color.Purple"%29%29%29
      (Rendering|Components|Decal|SetDecalMaterial (Variables|Decal|GetDecal) "/Game/Vehicle/Ability/InkEjection/M/MI_Decal_Purple.MI_Decal_Purple"))
    (:%28GameplayTags=%28%28TagName="Color.Red"%29%29%29
      (Rendering|Components|Decal|SetDecalMaterial (Variables|Decal|GetDecal) "/Game/Vehicle/Ability/InkEjection/M/MI_Decal_Red.MI_Decal_Red"))
    (:%28GameplayTags=%28%28TagName="Color.Yellow"%29%29%29
      (Rendering|Components|Decal|SetDecalMaterial (Variables|Decal|GetDecal) "/Game/Vehicle/Ability/InkEjection/M/MI_Decal_Yellow.MI_Decal_Yellow"))))