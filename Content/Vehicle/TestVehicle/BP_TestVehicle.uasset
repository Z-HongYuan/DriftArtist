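; Test vehicle pawn with physics driving and Gameplay Ability System abilities.
; Enhanced Input drives controls, resets, a single-use primary ability and EMP; airborne angular damping steadies the car.
; Looping timers auto-reset flipped cars and detect rear-wheel drift, triggering Niagara and passive ink ejection.
; Tick feeds rear slip angle into a gameplay effect via SetByCaller, while a watched attribute sets NeedCollision, whose RepNotify switches collision responses.
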(event Custom|AddMapping
  ;[0 1 0.5547] 添加InputMapping
  (bind _as玩家控制器 (Utilities|Casting|CastToPlayerController (Pawn|GetController)))
  (Input|AddMappingContext (PlayerController|LocalPlayerSubsystems|GetEnhancedInputLocalPlayerSubsystem _as玩家控制器) "/Game/Input/IMC_Default.IMC_Default" 0 "(bIgnoreAllPressedKeysUntilRelease=True,bForceImmediately=False,bNotifyUserSettings=False)")
  (Input|AddMappingContext (PlayerController|LocalPlayerSubsystems|GetEnhancedInputLocalPlayerSubsystem _as玩家控制器) "/Game/Input/IMC_DefaultAbility.IMC_DefaultAbility" 0 "(bIgnoreAllPressedKeysUntilRelease=True,bForceImmediately=False,bNotifyUserSettings=False)"))

(event Custom|Manual%20Reset
  ;[0.15 0.15 0.15 0.5] 重置车辆
  (Transformation|SetActorTransform (Math|Transform|MakeTransform (+ (Transformation|GetActorLocation) "0,0,50.000000") (Math|Rotator|MakeRotator 0.0 0.0 (.yaw (Transformation|GetActorRotation)))) false true)
  (Class|PrimitiveComponent|SetPhysicsAngularVelocityinDegrees (Variables|Character|GetMesh) "0, 0, 0" false "None")
  (Physics|SetPhysicsLinearVelocity (Variables|Character|GetMesh) "0, 0, 0" false "None"))

(event Custom|RemoveMapping
  ;[0.15 0.15 0.15 0.5] 未控制移除Mapping
  (bind _as玩家控制器 (Utilities|Casting|CastToPlayerController (Pawn|GetController)))
  (Input|RemoveMappingContext (PlayerController|LocalPlayerSubsystems|GetEnhancedInputLocalPlayerSubsystem _as玩家控制器) "/Game/Input/IMC_Default.IMC_Default" "(bIgnoreAllPressedKeysUntilRelease=True,bForceImmediately=False,bNotifyUserSettings=False)")
  (Input|RemoveMappingContext (PlayerController|LocalPlayerSubsystems|GetEnhancedInputLocalPlayerSubsystem _as玩家控制器) "/Game/Input/IMC_DefaultAbility.IMC_DefaultAbility" "(bIgnoreAllPressedKeysUntilRelease=True,bForceImmediately=False,bNotifyUserSettings=False)"))

(event Custom|ClearAbility
  (bind _outabilityhandles (GameplayAbilities|FindAllAbilitieswithTags (Variables|Default|GetAbilitySystemComponent) "(GameplayTags=((TagName=\"ActiveAbility\")))" true))
  (if (Utilities|Array|IsNotEmpty _outabilityhandles)
    (GameplayAbilities|ClearAbility (Variables|Default|GetAbilitySystemComponent) (Utilities|Array|Get(acopy) _outabilityhandles))))

(event Custom|CustomEvent_5
  ;[0.15 0.15 0.15 0.5] 重置车辆
  (Transformation|SetActorTransform (Math|Transform|MakeTransform (+ (Transformation|GetActorLocation) "0,0,50.000000") (Math|Rotator|MakeRotator 0.0 0.0 (.yaw (Transformation|GetActorRotation)))) false true)
  (Class|PrimitiveComponent|SetPhysicsAngularVelocityinDegrees (Variables|Character|GetMesh) "0, 0, 0" false "None")
  (Physics|SetPhysicsLinearVelocity (Variables|Character|GetMesh) "0, 0, 0" false "None"))

(event Input|EnhancedActionEvents|EnhancedInputActionIA_PrimaryAbility
  (params (ActionValue :type Float%20%28double-precision%29) (ElapsedSeconds :type Float%20%28double-precision%29) (TriggeredSeconds :type Float%20%28double-precision%29) (InputAction :type Input%20Action%20Object%20Reference :default "/Game/Input/AbilityAction/IA_PrimaryAbility.IA_PrimaryAbility"))
  (:Started
    (bind _outabilityhandles (GameplayAbilities|FindAllAbilitieswithTags (Variables|Default|GetAbilitySystemComponent) "(GameplayTags=((TagName=\"ActiveAbility\")))" true))
    (if (Utilities|Array|IsNotEmpty _outabilityhandles)
      (bind _returnvalue (Class|AbilitySystemComponent|TryActivateAbility (Variables|Default|GetAbilitySystemComponent) (Utilities|Array|Get(acopy) _outabilityhandles) true))
      (if _returnvalue
        (CallFunction|ClearAbility)))))

(event Input|EnhancedActionEvents|EnhancedInputActionIA_SecondaryAbility
  (params (ActionValue :type Float%20%28double-precision%29) (ElapsedSeconds :type Float%20%28double-precision%29) (TriggeredSeconds :type Float%20%28double-precision%29) (InputAction :type Input%20Action%20Object%20Reference :default "/Game/Input/AbilityAction/IA_SecondaryAbility.IA_SecondaryAbility"))
  (:Started
    (Abilities|TryActivateAbilitybyClass (Variables|Default|GetAbilitySystemComponent) "/Game/Vehicle/Ability/EMP/GA_EMP.GA_EMP_C" true)))

(event Input|EnhancedActionEvents|EnhancedInputActionIA_Throttle
  (params (ActionValue :type Float%20%28double-precision%29) (ElapsedSeconds :type Float%20%28double-precision%29) (TriggeredSeconds :type Float%20%28double-precision%29) (InputAction :type Input%20Action%20Object%20Reference :default "/Game/Input/MovementActions/IA_Throttle.IA_Throttle"))
  ;[0.15 0.15 0.15 0.5] 油门输入
  (:Triggered
    (Class|ChaosVehicleMovementComponent|SetThrottleInput (Class|DAVehiclePawnBase|GetVehicleCMC) ActionValue :!label _label))
  (:Completed
    (goto _label)))

(event Input|EnhancedActionEvents|EnhancedInputActionIA_Steering
  (params (ActionValue :type Float%20%28double-precision%29) (ElapsedSeconds :type Float%20%28double-precision%29) (TriggeredSeconds :type Float%20%28double-precision%29) (InputAction :type Input%20Action%20Object%20Reference :default "/Game/Input/MovementActions/IA_Steering.IA_Steering"))
  ;[0.05098 0.05098 0.05098] 转向输入
  (:Triggered
    (Class|ChaosVehicleMovementComponent|SetSteeringInput (Class|DAVehiclePawnBase|GetVehicleCMC) ActionValue :!label _label))
  (:Completed
    (goto _label)))

(event Input|EnhancedActionEvents|EnhancedInputActionIA_Brake
  (params (ActionValue :type Float%20%28double-precision%29) (ElapsedSeconds :type Float%20%28double-precision%29) (TriggeredSeconds :type Float%20%28double-precision%29) (InputAction :type Input%20Action%20Object%20Reference :default "/Game/Input/MovementActions/IA_Brake.IA_Brake"))
  (bind _returnvalue (Class|DAVehiclePawnBase|GetVehicleCMC))
  ;[0.15 0.15 0.15 0.5] 制动输入,并且开关刹车灯
  (:Triggered
    (Class|ChaosVehicleMovementComponent|SetBrakeInput _returnvalue ActionValue))
  (:Started
    (CallFunction|FlippedCheck true))
  (:Completed
    (Class|ChaosVehicleMovementComponent|SetBrakeInput _returnvalue ActionValue)
    (CallFunction|FlippedCheck false)))

(event Input|EnhancedActionEvents|EnhancedInputActionIA_Handbrake
  (params (ActionValue :type Boolean) (ElapsedSeconds :type Float%20%28double-precision%29) (TriggeredSeconds :type Float%20%28double-precision%29) (InputAction :type Input%20Action%20Object%20Reference :default "/Game/Input/MovementActions/IA_Handbrake.IA_Handbrake"))
  (bind _returnvalue (Class|DAVehiclePawnBase|GetVehicleCMC))
  ;[0.05098 0.05098 0.05098] 手刹输入,并且开关刹车灯
  (:Triggered
    (Class|ChaosVehicleMovementComponent|SetHandbrakeInput _returnvalue true)
    (CallFunction|FlippedCheck true))
  (:Completed
    (Class|ChaosVehicleMovementComponent|SetHandbrakeInput _returnvalue false)
    (CallFunction|FlippedCheck false)))

(event Input|EnhancedActionEvents|EnhancedInputActionIA_Reset
  (params (ActionValue :type Boolean) (ElapsedSeconds :type Float%20%28double-precision%29) (TriggeredSeconds :type Float%20%28double-precision%29) (InputAction :type Input%20Action%20Object%20Reference :default "/Game/Input/MovementActions/IA_Reset.IA_Reset"))
  ;[0.15 0.15 0.15 0.5] 重置车辆
  (:Started
    (CallFunction|ManualReset)
    (CallFunction|CustomEvent5)))

(event EventTick
  (params (DeltaSeconds :type Float%20%28single-precision%29))
  ;[0.05098 0.05098 0.05098] 车辆在空中时减少旋转
  (Class|PrimitiveComponent|SetAngularDamping (Variables|Character|GetMesh) (Math|Float|SelectFloat 0.0 3.0 (AI|Components|NavMovement|IsMovingonGround (Class|DAVehiclePawnBase|GetVehicleCMC))))
  (CallFunction|Debug)
  (Class|AbilitySystemComponent|UpdateActiveGameplayEffectSetbyCallerMagnitude (Variables|Default|GetAbilitySystemComponent) (stale EventBeginPlay _returnvalue_4) "(TagName=\"Data.SlipAngle\")" (Math|Float|MapRangeClamped (Math|Trig|RadiansToDegrees (/ (+ (.SlipAngle%20侧滑角度 (Utilities|GetVehicleWheelState 2)) (.SlipAngle%20侧滑角度 (Utilities|GetVehicleWheelState 3))) 2.0)) 0.0 5e+01 0.0 2.0)))

(event EventUnpossessed
  (params (OldController :type Controller%20Object%20Reference))
  ;[0.15 0.15 0.15 0.5] 未控制移除Mapping
  (CallFunction|RemoveMapping))

(event EventBeginPlay
  (bind _abilitysystemcomponent (Variables|Default|GetAbilitySystemComponent))
  ;[0.875 0 1] 转换并保存移动组件变量
  ; 并且每三秒检测一次当前车辆是否翻车
  (bind _returnvalue (Utilities|Time|SetTimerbyFunctionName 0 "Flipped Check" 3.0 true))
  (Variables|Default|SetFlipped%20Check%20Timer _returnvalue)
  (CallFunction|AttachMesh)
  (bind _returnvalue_2 (Utilities|Time|SetTimerbyFunctionName 0 "Check Drift" 0.2 true true))
  (Variables|Default|SetCheck%20Drift%20Timer _returnvalue_2)
  (bind _returnvalue_3 (Ability|GameplayEffect|AssignTagSetbyCallerMagnitude (GameplayEffects|MakeOutgoingSpec _abilitysystemcomponent "/Game/Vehicle/Ability/InkEjection/GE_.GE__C" 0.0 (GameplayEffects|MakeEffectContext _abilitysystemcomponent)) "(TagName=\"Data.SlipAngle\")" (Math|Float|MapRangeClamped (Math|Trig|RadiansToDegrees (/ (+ (.SlipAngle%20侧滑角度 (Utilities|GetVehicleWheelState 2)) (.SlipAngle%20侧滑角度 (Utilities|GetVehicleWheelState 3))) 2.0)) 0.0 5e+01 0.0 2.0)))
  (bind _returnvalue_4 (GameplayEffects|ApplyGameplayEffectSpecToSelf (Variables|Default|GetAbilitySystemComponent) _returnvalue_3)))

(event EventEndPlay
  (params (EndPlayReason :type EEndPlayReason%20Enum :default "Destroyed"))
  (Utilities|Time|ClearandInvalidateTimerbyHandle (Variables|Default|GetFlipped%20Check%20Timer))
  (Utilities|Time|ClearandInvalidateTimerbyHandle (Variables|Default|GetCheck%20Drift%20Timer)))

(event EventPossessed
  (params (NewController :type Controller%20Object%20Reference))
  ;[0 1 0.5547] 添加InputMapping
  (CallFunction|AddMapping)
  (bind _newvalue (Ability|Tasks|WaitForAttributeChanged 0 "(AttributeName=\"Collision\",Attribute=/Script/DriftArtist.DA_AttributeSetBase:Collision,AttributeOwner=\"/Script/CoreUObject.Class'/Script/DriftArtist.DA_AttributeSetBase'\")")
    (:Changed
      (CallFunction|设置碰撞 (> _newvalue 0.0)))))

(event Input|KeyboardEvents|LeftAlt
  (params (Key :type Key%20Structure :default "None"))
  (bind _returnvalue (Game|GetPlayerController 0))
  (bind _returnvalue_2 (Game|GetPlayerController 0))
  (:Pressed
    (Variables|/Script/Engine.PlayerController|SetbShowMouseCursor _returnvalue_2 true)
    (Input|SetInputModeUIOnly _returnvalue 0 "DoNotLock" false))
  (:Released
    (Variables|/Script/Engine.PlayerController|SetbShowMouseCursor _returnvalue_2 false)
    (Input|SetInputModeGameOnly _returnvalue false)))

(event Custom|设置碰撞
  (params (NeedCollision :type Boolean))
  (Variables|Default|SetNeed%20Collision NeedCollision))

(event Input|MouseEvents|LeftMouseButton
  (params (Key :type Key%20Structure))
  (bind _returnvalue (Class|DAVehiclePawnBase|GetVehicleCMC))
  (:Pressed
    (Class|ChaosWheeledVehicleMovementComponent|SetWheelSlipGraphMultiplier _returnvalue 0 0.0)
    (Class|ChaosWheeledVehicleMovementComponent|SetWheelSlipGraphMultiplier _returnvalue 1 0.0))
  (:Released
    (Class|ChaosWheeledVehicleMovementComponent|SetWheelSlipGraphMultiplier _returnvalue 0 1.0)
    (Class|ChaosWheeledVehicleMovementComponent|SetWheelSlipGraphMultiplier _returnvalue 0 1.0)))

(event Input|KeyboardEvents|Z
  (params (Key :type Key%20Structure)))

(event Input|KeyboardEvents|X
  (params (Key :type Key%20Structure)))

(fn ConstructionScript)

(fn AttachMesh
  (Transformation|AttachComponentToComponent (Variables|Default|GetSM_Wheel_Front_L_vehCar_vehicle06) (Variables|Character|GetMesh) "wheel_front_turn_l" "KeepWorld" "KeepWorld" "KeepWorld" true)
  (Transformation|AttachComponentToComponent (Variables|Default|GetSM_Wheel_Front_R_vehCar_vehicle06) (Variables|Character|GetMesh) "wheel_front_turn_r" "KeepWorld" "KeepWorld" "KeepWorld" true)
  (Transformation|AttachComponentToComponent (Variables|Default|GetSM_Wheel_Rear_L_vehCar_vehicle06) (Variables|Character|GetMesh) "wheel_rear_l" "KeepWorld" "KeepWorld" "KeepWorld" true)
  (Transformation|AttachComponentToComponent (Variables|Default|GetSM_Wheel_Rear_R_vehCar_vehicle06) (Variables|Character|GetMesh) "wheel_rear_r" "KeepWorld" "KeepWorld" "KeepWorld" true))

(fn FlippedCheck
  (params (Is%20Braking :type Boolean))
  (if (< (Math|Vector|DotProduct (Math|Vector|GetUpVector (Variables|Character|GetMesh)) "0.000000,0.000000,1.000000") -0.2)
    (if (Variables|Default|GetPrevious%20Flip%20Check)
      (CallFunction|ManualReset)
      (else
        (Variables|Default|SetPrevious%20Flip%20Check true)))
    (else
      (Variables|Default|SetPrevious%20Flip%20Check false))))

(fn CheckDrift
  (for _index (range 2 3)
    (if (and (.bInContact%20是否接触地面 (Utilities|GetVehicleWheelState _index)) (or (.bIsSlipping%20是否纵向打滑 (Utilities|GetVehicleWheelState _index)) (.bIsSkidding%20是否横向滑移 (Utilities|GetVehicleWheelState _index))))
      (Class|DAAbilitySystemComponent|AbilityInputTagPressed (Variables|Default|GetAbilitySystemComponent) (GameplayTags|MakeLiteralGameplayTag "(TagName=\"PassiveAbility.InkEjection\")"))
      (Components|Activation|Activate (Variables|Default|GetNiagara_BL) false)
      (else
        (Components|Activation|Deactivate (Variables|Default|GetNiagara_BR))))))

(fn Debug)

(fn OnRepNeedCollision
  (bind _mesh (Variables|Character|GetMesh))
  (if (Variables|Default|GetNeed%20Collision)
    (Collision|SetCollisionResponsetoChannel _mesh "ECC_Vehicle" "ECR_Ignore")
    (Collision|SetCollisionResponsetoChannel _mesh "ECC_GameTraceChannel1" "ECR_Ignore")
    (else
      (Collision|SetCollisionResponsetoChannel _mesh "ECC_Vehicle" "ECR_Block")
      (Collision|SetCollisionResponsetoChannel _mesh "ECC_GameTraceChannel1" "ECR_Overlap"))))