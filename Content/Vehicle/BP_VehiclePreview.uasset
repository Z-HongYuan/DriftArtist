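; Preview vehicle pawn that shows a saved engine mesh and takes basic keyboard driving input.
; AttachMesh attaches four wheel meshes to vehicle mesh sockets, keeping world transforms, in both the construction script and BeginPlay.
; BeginPlay then applies the engine static mesh from the "Default" save slot, if present.
; W, A and D set throttle and steering; releasing W applies negative throttle, and Space engages brake and handbrake without releasing them.
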(event EventBeginPlay
  (CallFunction|AttachMesh)
  ;[0.15 0.15 0.15 0.5] 拓展为应用设置
  (bind _returnvalue (SaveGame|DoesSaveGameExist "Default"))
  (if _returnvalue
    (bind _returnvalue_2 (SaveGame|LoadGamefromSlot "Default"))
    (bind _asbp_save_game (Utilities|Casting|CastToBP_SaveGame _returnvalue_2))
    (Components|StaticMesh|SetStaticMesh (Variables|Default|GetSM_EngineMesh) (Variables|/Game/SaveGame/BP_SaveGame.BP_SaveGame_C|GetNewVar _asbp_save_game))))

(event EventTick
  (params (DeltaSeconds :type Float%20%28single-precision%29)))

(event Input|KeyboardEvents|D
  (params (Key :type Key%20Structure :default "None"))
  (bind _returnvalue (Class|DAVehiclePawnBase|GetVehicleCMC))
  (:Pressed
    (Class|ChaosVehicleMovementComponent|SetSteeringInput _returnvalue -1.0))
  (:Released
    (Class|ChaosVehicleMovementComponent|SetSteeringInput _returnvalue 0.0)))

(event Input|KeyboardEvents|W
  (params (Key :type Key%20Structure :default "None"))
  (bind _returnvalue (Class|DAVehiclePawnBase|GetVehicleCMC))
  (:Pressed
    (Class|ChaosVehicleMovementComponent|SetThrottleInput _returnvalue 1.0))
  (:Released
    (Class|ChaosVehicleMovementComponent|SetThrottleInput _returnvalue -1.0)))

(event Input|KeyboardEvents|A
  (params (Key :type Key%20Structure :default "None"))
  (bind _returnvalue (Class|DAVehiclePawnBase|GetVehicleCMC))
  (:Pressed
    (Class|ChaosVehicleMovementComponent|SetSteeringInput _returnvalue 1.0))
  (:Released
    (Class|ChaosVehicleMovementComponent|SetSteeringInput _returnvalue 0.0)))

(event Input|KeyboardEvents|SpaceBar
  (params (Key :type Key%20Structure :default "None"))
  (:Pressed
    (Class|ChaosVehicleMovementComponent|SetHandbrakeInput (Variables|Default|GetVehicleMovementComponent) true)
    (Class|ChaosVehicleMovementComponent|SetBrakeInput (Variables|Default|GetVehicleMovementComponent) 1.0)))

(fn ConstructionScript
  (CallFunction|AttachMesh))

(fn AttachMesh
  (Transformation|AttachComponentToComponent (Variables|Default|GetSM_Wheel_FL) (Variables|Character|GetMesh) "wheel_front_turn_l" "KeepWorld" "KeepWorld" "KeepWorld" true)
  (Transformation|AttachComponentToComponent (Variables|Default|GetSM_Wheel_FR) (Variables|Character|GetMesh) "wheel_front_turn_r" "KeepWorld" "KeepWorld" "KeepWorld" true)
  (Transformation|AttachComponentToComponent (Variables|Default|GetSM_Wheel_BL) (Variables|Character|GetMesh) "wheel_rear_l" "KeepWorld" "KeepWorld" "KeepWorld" true)
  (Transformation|AttachComponentToComponent (Variables|Default|GetSM_Wheel_BR) (Variables|Character|GetMesh) "wheel_rear_r" "KeepWorld" "KeepWorld" "KeepWorld" true))