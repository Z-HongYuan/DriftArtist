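; Camera director Blueprint for the Gameplay Cameras system that drives a third-person camera for the test vehicle.
; Each run activates the third-person camera rig, then sets its field-of-view parameter from the vehicle's forward speed in MPH.
; A clamped range mapping widens the view as speed rises, and the current speed is printed to screen for debugging.
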(event EventRunCameraDirector
  (params (DeltaTime :type Float%20%28single-precision%29) (EvaluationContextOwner :type Object%20Object%20Reference) (Params :type Blueprint%20Camera%20Director%20Evaluation%20Params%20Structure%20%28by%20ref%29))
  (bind _returnvalue (Class|BlueprintCameraDirectorEvaluator|FindEvaluationContextOwnerActor "/Game/Vehicle/TestVehicle/BP_TestVehicle.BP_TestVehicle_C"))
  (bind _returnvalue_2 (Class|DAVehiclePawnBase|GetVehicleCMC _returnvalue))
  (bind _returnvalue_3 (Class|ChaosVehicleMovementComponent|GetForwardSpeedMPH _returnvalue_2))
  (Utilities|FlowControl|Sequence
    (:then_0
      (Class|BlueprintCameraDirectorEvaluator|ActivateCameraRig "/Game/Blueprints/CameraSystem/CRA_ThirdPerson.CRA_ThirdPerson" false))
    (:then_1
      (|SetCameraRigParameter (Class|BlueprintCameraDirectorEvaluator|GetInitialContextResult) (Math|Float|MapRangeClamped _returnvalue_3 0.0 1.2e+02 9e+01 1.2e+02))
      (Development|PrintString (Utilities|String|Append "前进速度MPH: " (Utilities|String|ToString(Float) _returnvalue_3)) true true "(R=0.000000,G=0.660000,B=1.000000,A=1.000000)" 0.0))))